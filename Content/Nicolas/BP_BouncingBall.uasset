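; Bouncing ball actor whose emissive sphere changes color and glow each time it registers a hit, for as long as it has HP.
; BeginPlay creates a dynamic instance of M_Emissive and assigns it to the Sphere.
; Each Sphere hit decrements HP and randomizes the material's Color and Intensity parameters, with color channels ranging far above 1.
; At zero HP further hits do nothing.
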(event OnComponentHit(Sphere)
  (params (HitComponent :type Primitive%20Component%20Object%20Reference) (OtherActor :type Actor%20Object%20Reference) (OtherComp :type Primitive%20Component%20Object%20Reference) (NormalImpulse :type Vector :default "0, 0, 0") (Hit :type Hit%20Result%20Structure%20%28by%20ref%29))
  (bind _mymaterial (Variables|Default|GetMyMaterial))
  (if (> (Variables|Default|GetHP) 0)
    (bind _result (Math|Integer|DecrementInt (Variables|Default|GetHP))
      (:%20%20
        (Variables|Default|SetHP _result)
        (Rendering|Material|SetVectorParameterValue _mymaterial "Color" (Math|Color|MakeColor (Math|Random|RandomFloatinRange 0.0 255.0) (Math|Random|RandomFloatinRange 0.0 255.0) (Math|Random|RandomFloatinRange 0.0 255.0)) :!class /Script/Engine.MaterialInstanceDynamic)
        (Rendering|Material|SetScalarParameterValue _mymaterial "Intensity" (Math|Random|RandomFloatinRange 5.0 15.0) :!class /Script/Engine.MaterialInstanceDynamic)))))

(event EventBeginPlay
  (bind _returnvalue (Rendering|Material|CreateDynamicMaterialInstance "/Game/Nicolas/Materials/M_Emissive.M_Emissive" "None" "None" :!class /Script/Engine.KismetMaterialLibrary))
  (Variables|Default|SetMyMaterial _returnvalue)
  (Rendering|Material|SetMaterial (Variables|Default|GetSphere) 0 _returnvalue))

(fn ConstructionScript)